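; BP_ChargedShot is a player shot, named as a charged attack, that damages actors tagged Enemy.
; On BeginPlay its Box collision is set to ignore the player pawn's instigator when moving.
; Box overlaps apply DamageAmount to enemies without destroying the shot, while blocking hits destroy it only against actors tagged Floor.
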(event OnComponentHit(Box)
  (params (HitComponent :type Primitive%20Component%20Object%20Reference) (OtherActor :type Actor%20Object%20Reference) (OtherComp :type Primitive%20Component%20Object%20Reference) (NormalImpulse :type Vector :default "0, 0, 0") (Hit :type Hit%20Result%20Structure%20%28by%20ref%29))
  (if (Utilities|IsValid OtherActor)
    (if (Actor|ActorHasTag OtherActor "Floor")
      (Actor|DestroyActor))))

(event OnComponentBeginOverlap(Box)
  (params (OverlappedComponent :type Primitive%20Component%20Object%20Reference) (OtherActor :type Actor%20Object%20Reference) (OtherComp :type Primitive%20Component%20Object%20Reference) (OtherBodyIndex :type Integer) (bFromSweep :type Boolean) (SweepResult :type Hit%20Result%20Structure%20%28by%20ref%29))
  ;[0.15 0.15 0.15 0.5] Checks if the collided target has the tag "Enemy" as deals 20 damage if so
  (if (Actor|ActorHasTag OtherActor "Enemy")
    (Game|Damage|ApplyDamage OtherActor (Variables|Default|GetDamageAmount) 0 0)))

(event EventBeginPlay
  (Collision|IgnoreActorwhenMoving (Variables|Default|GetBox) (Game|GetInstigator (Game|Player|GetPlayerPawn 0)) true))

(fn ConstructionScript)