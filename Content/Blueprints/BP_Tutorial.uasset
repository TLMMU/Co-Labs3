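; Tutorial trigger actor that updates on-screen tutorial text when the player enters its box.
; On BeginPlay it creates its own WBP_Tutorial widget for the first player controller and adds it to the viewport.
; When an actor tagged Player begins overlapping the Box, it passes its FirstBox, SecondBox and ThirdBox variables to the widget's UpdateText.
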(event OnComponentBeginOverlap(Box)
  (params (OverlappedComponent :type Primitive%20Component%20Object%20Reference) (OtherActor :type Actor%20Object%20Reference) (OtherComp :type Primitive%20Component%20Object%20Reference) (OtherBodyIndex :type Integer) (bFromSweep :type Boolean) (SweepResult :type Hit%20Result%20Structure%20%28by%20ref%29))
  (if (Actor|ActorHasTag OtherActor "Player")
    (Default|UpdateText (Variables|Default|GetWidgetVar) (Variables|Default|GetFirstBox) (Variables|Default|GetSecondBox) (Variables|Default|GetThirdBox))))

(event EventBeginPlay
  (bind _returnvalue (UserInterface|CreateWidget "/Game/Blueprints/WBP_Tutorial.WBP_Tutorial_C" (Game|GetPlayerController 0)))
  (bind _output_get (Variables|Default|SetWidgetVar _returnvalue))
  (UserInterface|Viewport|AddtoViewport _output_get 0))

(fn ConstructionScript)