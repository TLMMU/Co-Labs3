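; BP_PFS_Shot is a projectile that damages actors tagged Player on box overlap, then destroys itself.
; On BeginPlay its box ignores the instigator while moving.
; A helper function, not called in this graph, spawns BP_MetalChunks at a hit point and launches it along the randomly perturbed surface normal, setting only X and Z components.
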(event OnComponentBeginOverlap(Box)
  (params (OverlappedComponent :type Primitive%20Component%20Object%20Reference) (OtherActor :type Actor%20Object%20Reference) (OtherComp :type Primitive%20Component%20Object%20Reference) (OtherBodyIndex :type Integer) (bFromSweep :type Boolean) (SweepResult :type Hit%20Result%20Structure%20%28by%20ref%29))
  (if (Utilities|IsValid OtherActor)
    (if (Actor|ActorHasTag OtherActor "Player")
      (Game|Damage|ApplyDamage OtherActor (Variables|Default|GetDamageAmount) 0 0)
      (Actor|DestroyActor))))

(event EventBeginPlay
  (Collision|IgnoreActorwhenMoving (Variables|Default|GetBox) (Game|GetInstigator) true))

(fn ConstructionScript)

(fn GetChunkSpawn&Velocity
  (params (HitImpactPoint :type Vector) (HitImpactNormal :type Vector))
  (bind _returnvalue (Math|Random|RandomUnitVector))
  (bind (_x _y _z) (Math|Vector|BreakVector HitImpactPoint))
  (bind _returnvalue_2 (+ HitImpactNormal _returnvalue))
  (bind _returnvalue_3 (Math|Vector|Normalize _returnvalue_2))
  (bind _returnvalue_4 (Game|SpawnActorfromClass "/Game/Blueprints/BP_MetalChunks.BP_MetalChunks_C" (Math|Transform|MakeTransform (Math|Vector|MakeVector _x 0.0 _z) (Math|Vector|RotatorfromAxisandAngle HitImpactNormal 0.0) "1.000000,1.000000,1.000000") "Undefined" "MultiplyWithRoot" 0 0))
  (Physics|SetPhysicsLinearVelocity (Variables|/Game/Blueprints/BP_MetalChunks.BP_MetalChunks_C|GetBox _returnvalue_4) (Math|Vector|MakeVector (* (.x _returnvalue_3) 5e+02) 0.0 (* (.z _returnvalue_3) 5e+02)) true "None"))