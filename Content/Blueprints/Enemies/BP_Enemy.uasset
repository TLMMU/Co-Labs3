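; Enemy actor that damages the player on overlap and awards material to BP_ZD_Player when its health runs out.
; The EnemyMove timeline lerps the collision box between two points and rotates the sprite with the movement value.
; On death it removes box and sprite, stops the timeline and activates Niagara, feeding it the player's "Absorb" arrow position in local space each tick.
; The actor destroys itself when the effect finishes.
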(event OnSystemFinished(Niagara)
  (params (PSystem :type Niagara%20Component%20Object%20Reference))
  (Components|DestroyComponent (Variables|Default|GetNiagara))
  (Variables|Default|Setdestroyed false)
  (Actor|DestroyActor))

(event OnComponentBeginOverlap(Box)
  (params (OverlappedComponent :type Primitive%20Component%20Object%20Reference) (OtherActor :type Actor%20Object%20Reference) (OtherComp :type Primitive%20Component%20Object%20Reference) (OtherBodyIndex :type Integer) (bFromSweep :type Boolean) (SweepResult :type Hit%20Result%20Structure%20%28by%20ref%29))
  ;[0.15 0.15 0.15 0.5] Damages the player by a set amount upon collision
  (if (Utilities|IsValid OtherActor)
    (if (Components|ComponentHasTag OtherComp "Player")
      (Game|Damage|ApplyDamage OtherActor (Variables|Default|GetDamageAmount) 0 0))))

(event EventTick
  (params (DeltaSeconds :type Float%20%28single-precision%29))
  (bind _sprite (Variables|Default|GetSprite))
  (Utilities|FlowControl|Sequence
    (:then_0
      (if (Variables|Default|Getdestroyed)
        (if (< (Variables|Default|Gettick) 1.0)
          (Variables|Default|Settick (+ (Variables|Default|Gettick) 1.0))
          (bind _movement (Timeline|enemyMove Stop)
            (:Update
              (Transformation|SetRelativeLocation (Variables|Default|GetBox) (Math|Vector|Lerp(Vector) (Variables|Default|Getstart) (Variables|Default|Getend) _movement) false false)
              (Math|Float|CompareFloat _movement 0.0
                (:>
                  (Transformation|SetRelativeRotation _sprite "0.000000,0.000000,0.000000" false false))
                (:<
                  (Transformation|SetRelativeRotation _sprite "0.000000,180.000000,0.000000" false false))))))))
    (:then_1
      (if (Variables|Default|Getdestroyed)
        (Class|NiagaraComponent|SetVariablePosition (Variables|Default|GetNiagara) "Player_Pos" (Math|Transform|InverseTransformLocation (Transformation|GetWorldTransform (Variables|Default|GetNiagara)) (Transformation|GetWorldLocation (Utilities|Array|Get(acopy) (Actor|GetComponentsbyTag (Game|GetPlayerCharacter 0) "/Script/Engine.ArrowComponent" "Absorb")))))))))

(event EventBeginPlay
  (Niagara|SetNiagaraVariable(Float) (Variables|Default|GetNiagara) "Sprite_Size" 3.1)
  (Niagara|SetNiagaraVariable(Float) (Variables|Default|GetNiagara) "XYZ_Dimensions" 3.1))

(event Game|Damage|EventAnyDamage
  (params (Damage :type Float%20%28single-precision%29) (DamageType :type Damage%20Type%20Object%20Reference) (InstigatedBy :type Controller%20Object%20Reference) (DamageCauser :type Actor%20Object%20Reference))
  ;[0.15 0.15 0.15 0.5] Receives a value for damage from the shot blueprints and subtracts health accordingly. Destroys actor if health = 0
  (bind _output_get (Variables|Default|SetCurrentHealth (- (Variables|Default|GetCurrentHealth) Damage)))
  (if (<= _output_get (Variables|Default|GetNoHealth))
    (Variables|Default|Setdestroyed true)
    (Components|DestroyComponent (Variables|Default|GetBox))
    (Components|DestroyComponent (Variables|Default|GetSprite))
    (Components|Activation|Activate (Variables|Default|GetNiagara) false)
    (bind _asbp_zd_player (Utilities|Casting|CastToBP_ZD_Player (Game|GetPlayerCharacter 0)))
    (Variables|/Game/Blueprints/Player/BP_ZD_Player.BP_ZD_Player_C|SetcurrentMCount _asbp_zd_player (+ (Variables|/Game/Blueprints/Player/BP_ZD_Player.BP_ZD_Player_C|GetcurrentMCount _asbp_zd_player) (Variables|Default|GetmaterialGain)))))

(fn ConstructionScript)