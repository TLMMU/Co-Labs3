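; Patrolling sprite enemy that damages the player on contact and awards materials when killed.
; Two timelines alternate to drive movement input along the X axis, each setting the sprite's facing and starting the other when finished.
; Box overlap damages Player-tagged components; incoming damage reduces health.
; At zero health it removes box and sprite, activates Niagara and credits BP_ZD_Player, while a one-time Tick gate stops both timelines.
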(event OnComponentBeginOverlap(Box)
  (params (OverlappedComponent :type Primitive%20Component%20Object%20Reference) (OtherActor :type Actor%20Object%20Reference) (OtherComp :type Primitive%20Component%20Object%20Reference) (OtherBodyIndex :type Integer) (bFromSweep :type Boolean) (SweepResult :type Hit%20Result%20Structure%20%28by%20ref%29))
  ;[0.15 0.15 0.15 0.5] Damages the player by a set amount upon collision
  (if (Utilities|IsValid OtherActor)
    (if (Components|ComponentHasTag OtherComp "Player")
      (Game|Damage|ApplyDamage OtherActor (Variables|Default|GetDamage%20Amount) 0 0))))

(event Custom|ReverseWalk
  (bind _movement (Timeline|EnemyMovementRight PlayFromStart)
    (:Update
      (Pawn|Input|AddMovementInput "1.000000,0.000000,0.000000" _movement false)
      (Transformation|SetRelativeRotation (Variables|Default|GetSprite) "0, 0, 0" false false))
    (:Finished
      (CallFunction|StartWalk))))

(event Custom|StartWalk
  (bind _movement (Timeline|EnemyMovementLeft PlayFromStart)
    (:Update
      (Pawn|Input|AddMovementInput "1.000000,0.000000,0.000000" _movement false)
      (Transformation|SetRelativeRotation (Variables|Default|GetSprite) "0.000000,180.000000,0.000000" false false))
    (:Finished
      (CallFunction|ReverseWalk))))

(event EventTick
  (params (DeltaSeconds :type Float%20%28single-precision%29))
  (bind _sprite (Variables|Default|GetSprite))
  (if (Variables|Default|Getdestroyed)
    (if (< (Variables|Default|Gettick) 1.0)
      (Variables|Default|Settick 1.0)
      (Utilities|FlowControl|Sequence
        (:then_0
          (bind _movement (Timeline|EnemyMovementLeft Stop)
            (:Update
              (Pawn|Input|AddMovementInput "1.000000,0.000000,0.000000" _movement false)
              (Transformation|SetRelativeRotation _sprite "0.000000,180.000000,0.000000" false false))
            (:Finished
              (CallFunction|ReverseWalk))))
        (:then_1
          (bind _movement_2 (Timeline|EnemyMovementRight Stop)
            (:Update
              (Pawn|Input|AddMovementInput "1.000000,0.000000,0.000000" _movement_2 false)
              (Transformation|SetRelativeRotation _sprite "0, 0, 0" false false))
            (:Finished
              (CallFunction|StartWalk))))))))

(event EventBeginPlay
  (CallFunction|StartWalk))

(event Game|Damage|EventAnyDamage
  (params (Damage :type Float%20%28single-precision%29) (DamageType :type Damage%20Type%20Object%20Reference) (InstigatedBy :type Controller%20Object%20Reference) (DamageCauser :type Actor%20Object%20Reference))
  ;[0.15 0.15 0.15 0.5] Receives a value for damage from the shot blueprints and subtracts health accordingly. Destroys actor if health = 0
  (bind _output_get (Variables|Default|SetCurrentHealth (- (Variables|Default|GetCurrentHealth) Damage)))
  (if (<= _output_get (Variables|Default|GetNo%20Health))
    (Variables|Default|Setdestroyed true)
    (Components|DestroyComponent (Variables|Default|GetBox))
    (Components|DestroyComponent (Variables|Default|GetSprite))
    (Components|Activation|Activate (Variables|Default|GetNiagara) false)
    (bind _asbp_zd_player (Utilities|Casting|CastToBP_ZD_Player (Game|GetPlayerCharacter 0)))
    (Variables|/Game/Blueprints/Player/BP_ZD_Player.BP_ZD_Player_C|SetcurrentMCount _asbp_zd_player (+ (Variables|/Game/Blueprints/Player/BP_ZD_Player.BP_ZD_Player_C|GetcurrentMCount _asbp_zd_player) (Variables|Default|GetMaterial%20Gain)))))

(fn ConstructionScript)