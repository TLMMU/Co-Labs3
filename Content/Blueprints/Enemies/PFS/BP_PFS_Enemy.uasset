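; 2D patrolling ranged enemy that damages the player on contact and grants materials to the player when killed.
; A looping timer reverses its walk direction, while Tick flips the sprite and rotate point by X velocity.
; When the player enters the detection box, it stops, plays an attack animation and tracks their position.
; Two seconds later it fires a BP_PFS_Shot along that aim and resumes walking.
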(event OnComponentBeginOverlap(Box)
  (params (OverlappedComponent :type Primitive%20Component%20Object%20Reference) (OtherActor :type Actor%20Object%20Reference) (OtherComp :type Primitive%20Component%20Object%20Reference) (OtherBodyIndex :type Integer) (bFromSweep :type Boolean) (SweepResult :type Hit%20Result%20Structure%20%28by%20ref%29))
  ;[0.15 0.15 0.15 0.5] Damages the player by a set amount upon collision
  (if (Utilities|IsValid OtherActor)
    (if (Components|ComponentHasTag OtherComp "Player")
      (Game|Damage|ApplyDamage OtherActor (Variables|Default|GetDamageAmount) 0 0))))

(event OnComponentBeginOverlap(DetectionBox)
  (params (OverlappedComponent :type Primitive%20Component%20Object%20Reference) (OtherActor :type Actor%20Object%20Reference) (OtherComp :type Primitive%20Component%20Object%20Reference) (OtherBodyIndex :type Integer) (bFromSweep :type Boolean) (SweepResult :type Hit%20Result%20Structure%20%28by%20ref%29))
  ;[0.15 0.15 0.15 0.5] Player Detection.
  (bind _ascapsule_collision (Utilities|Casting|CastToCapsuleComponent OtherComp))
  (if (Utilities|IsValid OtherActor)
    (Variables|Default|SetOtherActor OtherActor)
    (if (Components|ComponentHasTag _ascapsule_collision "Player")
      (Variables|Default|SetStopMovement true)
      (Class|PaperZDAnimInstance|JumptoNode (Variables|/Script/PaperZD.PaperZDAnimationComponent|GetAnimInstance (Variables|Default|GetAnimationComponent)) "PFSAttack" "None")
      (Variables|Default|SetAttackingPlayer true)
      (Utilities|Time|SetTimerbyEvent (delegate Custom|StopAttackingPFS) 2.0))))

(event Custom|StopAttackingPFS
  ;[0.15 0.15 0.15 0.5] Player Detection.
  (Variables|Default|SetStopMovement false)
  (Variables|Default|SetAttackingPlayer false)
  (Game|SpawnActorfromClass "/Game/Blueprints/Projectiles/BP_PFS_Shot.BP_PFS_Shot_C" (Math|Transform|MakeTransform (Transformation|GetWorldLocation (Variables|Default|GetProjectilePoint)) (Variables|Default|GetLastKnownPlayerRot) "0.300000,0.300000,0.300000") "Undefined" "MultiplyWithRoot" 0 0))

(event Custom|EnemyMovementPFS
  (Variables|Default|SetScaleValue (* (Variables|Default|GetScaleValue) -1.0)))

(event Custom|GetPlayerPosPFS
  (if (Variables|Default|GetAttackingPlayer)
    (Variables|Default|SetLastKnownPlayerRot (Math|Rotator|FindLookatRotation (Transformation|GetWorldLocation (Variables|Default|GetProjectilePoint)) (Transformation|GetWorldLocation (Variables|/Script/Engine.Actor|GetRootComponent (Variables|Default|GetOtherActor)))))))

(event EventTick
  (params (DeltaSeconds :type Float%20%28single-precision%29))
  (bind _rotatepoint (Variables|Default|GetRotatePoint))
  (bind _sprite (Variables|Default|GetSprite))
  (CallFunction|GetPlayerPosPFS)
  (if (not (Variables|Default|GetStopMovement))
    (Pawn|Input|AddMovementInput (Transformation|GetActorForwardVector) (/ (Variables|Default|GetScaleValue) 2.0) false)
    (Math|Float|CompareFloat (.x (Variables|/Script/Engine.MovementComponent|GetVelocity (Variables|Character|GetCharacterMovement))) 0.0
      (:>
        (Transformation|SetRelativeRotation _sprite "0.000000,180.000000,0.000000" false false)
        (Transformation|SetWorldRotation _rotatepoint "0.000000,180.000000,0.000000" false false))
      (:<
        (Transformation|SetRelativeRotation _sprite "0, 0, 0" false false)
        (Transformation|SetWorldRotation _rotatepoint "0, 0, 0" false false)))))

(event Game|Damage|EventAnyDamage
  (params (Damage :type Float%20%28single-precision%29) (DamageType :type Damage%20Type%20Object%20Reference) (InstigatedBy :type Controller%20Object%20Reference) (DamageCauser :type Actor%20Object%20Reference))
  ;[0.15 0.15 0.15 0.5] Receives a value for damage from the shot blueprints and subtracts health accordingly. Destroys actor if health = 0
  (bind _output_get (Variables|Default|SetCurrentHealth (- (Variables|Default|GetCurrentHealth) Damage)))
  (if (<= _output_get (Variables|Default|GetNoHealth))
    (Variables|Default|Setdestroyed true)
    (bind _asbp_zd_player (Utilities|Casting|CastToBP_ZD_Player (Game|GetPlayerCharacter 0)))
    (Variables|/Game/Blueprints/Player/BP_ZD_Player.BP_ZD_Player_C|SetcurrentMCount _asbp_zd_player (+ (Variables|/Game/Blueprints/Player/BP_ZD_Player.BP_ZD_Player_C|GetcurrentMCount _asbp_zd_player) (Variables|Default|GetMaterialGain)))
    (Actor|DestroyActor)))

(event EventBeginPlay
  (Utilities|Time|SetTimerbyEvent (delegate Custom|EnemyMovementPFS) (Variables|Default|GetWalkTime) true))

(fn ConstructionScript)