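; BP_NewEnemy is a sprite-based enemy that patrols back and forth along the world X axis without end.
; BeginPlay starts two timelines that restart each other on finish, one for each walk direction.
; Each timeline's Movement track scales the movement input, while the sprite's relative rotation is set every update to flip it for that direction.
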(event Custom|ReverseWalk
  (bind _movement (Timeline|EnemyMovementRight PlayFromStart)
    (:Update
      (Pawn|Input|AddMovementInput "1.000000,0.000000,0.000000" _movement false)
      (Transformation|SetRelativeRotation (Variables|Default|GetSprite) "0, 0, 0" false false))
    (:Finished
      (CallFunction|StartWalk))))

(event Custom|StartWalk
  (bind _movement (Timeline|EnemyMovementLeft PlayFromStart)
    (:Update
      (Pawn|Input|AddMovementInput "1.000000,0.000000,0.000000" _movement false)
      (Transformation|SetRelativeRotation (Variables|Default|GetSprite) "0.000000,180.000000,0.000000" false false))
    (:Finished
      (CallFunction|ReverseWalk))))

(event EventBeginPlay
  (CallFunction|StartWalk))

(fn ConstructionScript)