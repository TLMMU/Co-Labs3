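; SC enemy that patrols back and forth, damages the player on contact, and attacks at range with a spawned vine.
; A looping timer reverses movement, while Tick flips the sprite to match velocity.
; Player detection halts it and starts the attack animation, with a warning marker trailing the player via VInterpTo.
; Chained timers freeze tracking, then spawn BP_VineAttack below the last position and resume patrol; death awards materials to the player.
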(event OnComponentBeginOverlap(Box)
  (params (OverlappedComponent :type Primitive%20Component%20Object%20Reference) (OtherActor :type Actor%20Object%20Reference) (OtherComp :type Primitive%20Component%20Object%20Reference) (OtherBodyIndex :type Integer) (bFromSweep :type Boolean) (SweepResult :type Hit%20Result%20Structure%20%28by%20ref%29))
  ;[0.15 0.15 0.15 0.5] Damages the player by a set amount upon collision
  (if (Utilities|IsValid OtherActor)
    (if (Components|ComponentHasTag OtherComp "Player")
      (Game|Damage|ApplyDamage OtherActor (Variables|Default|GetDamageAmount) 0 0))))

(event OnComponentBeginOverlap(PlayerDetection)
  (params (OverlappedComponent :type Primitive%20Component%20Object%20Reference) (OtherActor :type Actor%20Object%20Reference) (OtherComp :type Primitive%20Component%20Object%20Reference) (OtherBodyIndex :type Integer) (bFromSweep :type Boolean) (SweepResult :type Hit%20Result%20Structure%20%28by%20ref%29))
  ;[0.15 0.15 0.15 0.5] This detects the player when they overlap and opens the gate for the vine "searching".
  (bind _ascapsule_collision (Utilities|Casting|CastToCapsuleComponent OtherComp))
  (if (Utilities|IsValid OtherActor)
    (Variables|Default|SetOtherActor OtherActor)
    (if (Components|ComponentHasTag _ascapsule_collision "Player")
      (Variables|Default|SetStopMovement true)
      (Class|PaperZDAnimInstance|JumptoNode (Variables|/Script/PaperZD.PaperZDAnimationComponent|GetAnimInstance (Variables|Default|GetAnimationComponent)) "SCAttack" "None")
      (Variables|Default|SetAttackingPlayer true)
      (Utilities|Time|SetTimerbyEvent (delegate Custom|StopAttackingSC) 3.0))))

(event Custom|StopAttackingSC
  ;[0.15 0.15 0.15 0.5] This detects the player when they overlap and opens the gate for the vine "searching".
  (Variables|Default|SetAttackingPlayer false)
  (Utilities|Time|SetTimerbyEvent (delegate Custom|SpawnVine) 2.0))

(event Custom|EnemyMovementSC
  (Variables|Default|SetScaleValue (* (Variables|Default|GetScaleValue) -1.0)))

(event Custom|SpawnVine
  (bind _lastpos (Variables|Default|GetLastPos))
  ;[0.15 0.15 0.15 0.5] This detects the player when they overlap and opens the gate for the vine "searching".
  (Rendering|SetVisibility (Variables|Default|GetWarning) false false)
  (Variables|Default|SetStopMovement false)
  (Game|SpawnActorfromClass "/Game/Blueprints/BP_VineAttack.BP_VineAttack_C" (Math|Transform|MakeTransform (Math|Vector|MakeVector (.x _lastpos) (.y _lastpos) (- (.z _lastpos) 8e+01)) "0, 0, 0" "0.300000,0.300000,0.300000") "Undefined" "MultiplyWithRoot" 0 0))

(event Custom|GetPlayerPos
  (bind _returnvalue (Utilities|Time|GetWorldDeltaSeconds))
  (bind _otheractor (Variables|Default|GetOtherActor))
  (bind _warning (Variables|Default|GetWarning))
  (bind _returnvalue_2 (Transformation|GetWorldLocation _warning))
  (bind _rootcomponent (Variables|/Script/Engine.Actor|GetRootComponent _otheractor))
  (bind _returnvalue_3 (Transformation|GetWorldLocation _rootcomponent))
  (bind _returnvalue_4 (+ (.y _returnvalue_3) 1e+01))
  (bind _returnvalue_5 (+ (.z _returnvalue_3) 6e+01))
  (bind _returnvalue_6 (Math|Interpolation|VInterpTo _returnvalue_2 (Math|Vector|MakeVector (.x _returnvalue_3) _returnvalue_4 _returnvalue_5) _returnvalue 3.0))
  ;[0.15 0.15 0.15 0.5] This is the vine "searching" that lags behind the player's position.
  (if (Variables|Default|GetAttackingPlayer)
    (Variables|Default|SetSearchTime (Math|Float|Clamp(Float) (- (Variables|Default|GetSearchTime) (Utilities|Time|GetWorldDeltaSeconds)) 0.0 (Variables|Default|GetSearchTime)))
    (Variables|Default|SetLastPos _returnvalue_6)
    (Transformation|SetWorldLocation (Variables|Default|GetWarning) _returnvalue_6 false false)
    (Rendering|SetVisibility (Variables|Default|GetWarning) true false)
    (if (<= (Variables|Default|GetSearchTime) 0.0)
      _)))

(event EventTick
  (params (DeltaSeconds :type Float%20%28single-precision%29))
  (bind _sprite (Variables|Default|GetSprite))
  (CallFunction|GetPlayerPos)
  (if (not (Variables|Default|GetStopMovement))
    (Pawn|Input|AddMovementInput (Transformation|GetActorForwardVector) (/ (Variables|Default|GetScaleValue) 2.0) false)
    (Math|Float|CompareFloat (.x (Variables|/Script/Engine.MovementComponent|GetVelocity (Variables|Character|GetCharacterMovement))) 0.0
      (:>
        (Transformation|SetRelativeRotation _sprite "0.000000,180.000000,0.000000" false false))
      (:<
        (Transformation|SetRelativeRotation _sprite "0, 0, 0" false false)))))

(event Game|Damage|EventAnyDamage
  (params (Damage :type Float%20%28single-precision%29) (DamageType :type Damage%20Type%20Object%20Reference) (InstigatedBy :type Controller%20Object%20Reference) (DamageCauser :type Actor%20Object%20Reference))
  ;[0.15 0.15 0.15 0.5] Receives a value for damage from the shot blueprints and subtracts health accordingly. Destroys actor if health = 0
  (bind _output_get (Variables|Default|SetCurrentHealth (- (Variables|Default|GetCurrentHealth) Damage)))
  (if (<= _output_get (Variables|Default|GetNoHealth))
    (Variables|Default|Setdestroyed true)
    (bind _asbp_zd_player (Utilities|Casting|CastToBP_ZD_Player (Game|GetPlayerCharacter 0)))
    (Variables|/Game/Blueprints/Player/BP_ZD_Player.BP_ZD_Player_C|SetcurrentMCount _asbp_zd_player (+ (Variables|/Game/Blueprints/Player/BP_ZD_Player.BP_ZD_Player_C|GetcurrentMCount _asbp_zd_player) (Variables|Default|GetMaterialGain)))
    (Actor|DestroyActor)))

(event EventBeginPlay
  (Utilities|Time|SetTimerbyEvent (delegate Custom|EnemyMovementSC) (Variables|Default|GetWalkTime) true))

(fn ConstructionScript)