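; BP_VineAttack is a one-shot 2D vine attack actor that damages the player on contact.
; On BeginPlay it turns off flipbook looping and jumps the PaperZD AnimInstance to the "Vines" node.
; Overlaps on the flipbook apply DamageAmount to actors whose overlapping component carries the "Player" tag.
; The actor destroys itself when the flipbook finishes playing.
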(event OnFinishedPlaying(PaperFlipbook)
  (Actor|DestroyActor))

(event OnComponentBeginOverlap(PaperFlipbook)
  (params (OverlappedComponent :type Primitive%20Component%20Object%20Reference) (OtherActor :type Actor%20Object%20Reference) (OtherComp :type Primitive%20Component%20Object%20Reference) (OtherBodyIndex :type Integer) (bFromSweep :type Boolean) (SweepResult :type Hit%20Result%20Structure%20%28by%20ref%29))
  (if (Utilities|IsValid OtherActor)
    (if (Components|ComponentHasTag OtherComp "Player")
      (Game|Damage|ApplyDamage OtherActor (Variables|Default|GetDamageAmount) 0 0))))

(event EventBeginPlay
  (Components|Timeline|SetLooping (Variables|Default|GetPaperFlipbook) false)
  (Class|PaperZDAnimInstance|JumptoNode (Variables|/Script/PaperZD.PaperZDAnimationComponent|GetAnimInstance (Variables|Default|GetPaperZDAnimation)) "Vines" "None"))

(fn ConstructionScript)