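; BP_Tutorial is a level-placed trigger that shows tutorial text to the player while inside its box.
; On BeginPlay each instance creates its own WBP_Tutorial widget and adds it to the viewport.
; When a component tagged Player enters the box, it passes four box variables to the widget's UpdateText, and clears the text when that component leaves.
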(event OnComponentBeginOverlap(Box)
  (params (OverlappedComponent :type Primitive%20Component%20Object%20Reference) (OtherActor :type Actor%20Object%20Reference) (OtherComp :type Primitive%20Component%20Object%20Reference) (OtherBodyIndex :type Integer) (bFromSweep :type Boolean) (SweepResult :type Hit%20Result%20Structure%20%28by%20ref%29))
  (if (Components|ComponentHasTag OtherComp "Player")
    (Default|UpdateText (Variables|Default|GetWidgetVar) (Variables|Default|GetFirstBox) (Variables|Default|GetSecondBox) (Variables|Default|GetThirdBox) (Variables|Default|GetFourthBox))))

(event OnComponentEndOverlap(Box)
  (params (OverlappedComponent :type Primitive%20Component%20Object%20Reference) (OtherActor :type Actor%20Object%20Reference) (OtherComp :type Primitive%20Component%20Object%20Reference) (OtherBodyIndex :type Integer))
  (if (Components|ComponentHasTag OtherComp "Player")
    (Default|ClearText (Variables|Default|GetWidgetVar))))

(event EventBeginPlay
  (bind _returnvalue (UserInterface|CreateWidget "/Game/Blueprints/Widgets/WBP_Tutorial.WBP_Tutorial_C" (Game|GetPlayerController 0)))
  (bind _output_get (Variables|Default|SetWidgetVar _returnvalue))
  (UserInterface|Viewport|AddtoViewport _output_get 0))

(fn ConstructionScript)