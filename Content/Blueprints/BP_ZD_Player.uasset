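; Side-scrolling player character that moves along world X, jumps and can toggle between a sprite form and a blood particle effect.
; BeginPlay creates the UI widget and adds the Enhanced Input mapping context.
; Tick flips the sprite to face horizontal velocity and opens TestMap when Hp reaches zero.
; The transform input uses a FlipFlop to swap visibility and activation of Sprite and Blood, reinitializing the effect on return.
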(event Custom|PlayerRotation
  (bind _sprite (Variables|Default|GetSprite))
  (Math|Float|CompareFloat (.x (Variables|/Script/Engine.MovementComponent|GetVelocity (Variables|Character|GetCharacterMovement))) 0.0
    (:>
      (Transformation|SetRelativeRotation _sprite "0, 0, 0" false false))
    (:<
      (Transformation|SetRelativeRotation _sprite "0.000000,180.000000,0.000000" false false))))

(event Input|EnhancedActionEvents|EnhancedInputActionIA_Move
  (params (ActionValue :type Float%20%28double-precision%29) (ElapsedSeconds :type Float%20%28double-precision%29) (TriggeredSeconds :type Float%20%28double-precision%29) (InputAction :type Input%20Action%20Object%20Reference :default "/Game/Input/IA_Move.IA_Move"))
  (Pawn|Input|AddMovementInput "1.000000,0.000000,0.000000" ActionValue false))

(event Input|EnhancedActionEvents|EnhancedInputActionIA_Jump
  (params (ActionValue :type Float%20%28double-precision%29) (ElapsedSeconds :type Float%20%28double-precision%29) (TriggeredSeconds :type Float%20%28double-precision%29) (InputAction :type Input%20Action%20Object%20Reference :default "/Game/Input/IA_Jump.IA_Jump"))
  (:Triggered
    (Character|Jump))
  (:Completed
    (Character|StopJumping)))

(event Input|EnhancedActionEvents|EnhancedInputActionIA_Transform
  (params (ActionValue :type Float%20%28double-precision%29) (ElapsedSeconds :type Float%20%28double-precision%29) (TriggeredSeconds :type Float%20%28double-precision%29) (InputAction :type Input%20Action%20Object%20Reference :default "/Game/Input/IA_Transform.IA_Transform"))
  (bind _sprite (Variables|Default|GetSprite))
  (bind _blood (Variables|Default|GetBlood))
  (bind _blood_2 (Variables|Default|GetBlood))
  (bind _sprite_2 (Variables|Default|GetSprite))
  (Utilities|FlowControl|FlipFlop
    (:A
      (Rendering|SetVisibility _sprite_2 false false)
      (Components|Activation|SetActive _sprite_2 false false)
      (Rendering|SetVisibility _blood_2 true false)
      (Components|Activation|SetActive _blood_2 true false))
    (:B
      (Niagara|ReinitializeSystem (Variables|Default|GetBlood))
      (Rendering|SetVisibility _blood false false)
      (Components|Activation|SetActive _blood false false)
      (Rendering|SetVisibility _sprite true false)
      (Components|Activation|SetActive _sprite true false))))

(event EventBeginPlay
  (bind _returnvalue (Game|GetPlayerController 0))
  (bind _returnvalue_2 (PlayerController|LocalPlayerSubsystems|GetEnhancedInputLocalPlayerSubsystem _returnvalue))
  (Utilities|FlowControl|Sequence
    (:then_0
      (bind _returnvalue_3 (UserInterface|CreateWidget "/Game/Blueprints/Widgets/Widget_UI.Widget_UI_C"))
      (UserInterface|Viewport|AddtoViewport _returnvalue_3 0))
    (:then_1
      (Utilities|IsValid _returnvalue_2
        (:Is%20Valid
          (Input|AddMappingContext _returnvalue_2 "/Game/Input/IMC_Player.IMC_Player" 0 "(bIgnoreAllPressedKeysUntilRelease=True,bForceImmediately=False,bNotifyUserSettings=False)"))))))

(event EventTick
  (params (DeltaSeconds :type Float%20%28single-precision%29))
  (Utilities|FlowControl|Sequence
    (:then_0
      (if (<= (Variables|Default|Gethp) 0)
        (Game|OpenLevel(byObjectReference) "/Game/Maps/TestMap.TestMap")))
    (:then_1
      (CallFunction|PlayerRotation))))

(fn ConstructionScript)